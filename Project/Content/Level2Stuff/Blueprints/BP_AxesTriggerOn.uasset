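; BP_AxesTriggerOn is a Level 2 trigger actor that moves its Box to a target position once the player touches it.
; An overlap with BP_Player sets IsTriggered, which is cleared only at BeginPlay, so the trigger never reverts during play.
; While triggered, Tick lerps Box from its current location toward TriggeredPosition by LerpAlpha, giving an eased, frame-rate-dependent slide without sweep.
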(event `self.ReceiveBeginPlay`
  (set `self.isTriggered` false))

(event `self.ReceiveActorBeginOverlap`
  (params (OtherActor :type "Actor Object Reference"))
  ;[1 1 1] Overlap Events
  (cast `/Game/Blueprints/BP_Player` OtherActor)
  (set `self.isTriggered` true))

(event `self.ReceiveTick`
  (params (DeltaSeconds :type "Float (single-precision)"))
  (if (`self.isTriggered`)
    (`SceneComponent.K2_SetWorldLocation` (`self.Box`) (`KismetMathLibrary.VLerp` (`SceneComponent.K2_GetComponentLocation` (`self.Box`)) (`self.triggeredPosition`) (`self.lerpAlpha`)) false false)))

(fn `UserConstructionScript`)