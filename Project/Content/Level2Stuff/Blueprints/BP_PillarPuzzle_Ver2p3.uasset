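; A rotating pillar puzzle piece that the player turns in fixed increments by pressing E while inside its overlap area.
; Each press adds an increment to a target rotation, wrapping yaw at a full turn, and Tick lerps the pivot toward it.
; A timer enforces a delay between presses.
; PuzzleSolved is set every frame by comparing the target rotation to the correct one within a tolerance.
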(event `self.ReceiveBeginPlay`
  (set `self.destinationRotation` (`SceneComponent.K2_GetComponentRotation` (`self.Pivot`))))

(event `self.ReceiveTick`
  (params (DeltaSeconds :type "Float (single-precision)"))
  (bind _yaw (.yaw (`self.destinationRotation`)))
  (bind _yaw_2 (.yaw (`self.destinationRotation`)))
  ;[1 1 1] Update
  (`|ExecutionSequence`
    (:`then_0`
      ;[1 1 1] Rotate Object
      (`SceneComponent.K2_SetWorldRotation` (`self.Pivot`) (`KismetMathLibrary.RLerp` (`SceneComponent.K2_GetComponentRotation` (`self.Pivot`)) (`self.destinationRotation`) (`self.lerpAlpha`) true) false false)
      (if (and (`PlayerController.IsInputKeyDown` (`GameplayStatics.GetPlayerController` 0) "E") (`self.isInRange`) (`self.isWaitTimeOver`))
        (set `self.isWaitTimeOver` false)
        (set `self.destinationRotation` (`KismetMathLibrary.ComposeRotators` (`self.destinationRotation`) (`self.incrementRotation`)))
        (if (>= _yaw_2 360.0)
          (set `self.destinationRotation` (`KismetMathLibrary.MakeRotator` (.roll (`self.destinationRotation`)) (.pitch (`self.destinationRotation`)) (- _yaw_2 360.0)))
          (elif (<= _yaw -360.0)
            (set `self.destinationRotation` (`KismetMathLibrary.MakeRotator` (.roll (`self.destinationRotation`)) (.pitch (`self.destinationRotation`)) (+ _yaw 360.0)))))))
    (:`then_1`
      ;[1 1 1] Wait Timer
      (if (`self.isWaitTimeOver`)
        _
        (elif (>= (`self.waitTimer`) (`self.totalWaitTime`))
          (set `self.waitTimer` 0.0)
          (set `self.isWaitTimeOver` true)
          (else
            (set `self.waitTimer` (+ (`GameplayStatics.GetWorldDeltaSeconds`) (`self.waitTimer`)))))))
    (:`then_2`
      ;[1 1 1] update puzzle solved
      (if (== (`self.destinationRotation`) (`self.correctRotation`) :`ErrorTolerance` 15.0)
        (set `self.puzzleSolved` true)
        (else
          (set `self.puzzleSolved` false))))))

(event `self.ReceiveActorBeginOverlap`
  (params (OtherActor :type "Actor Object Reference"))
  ;[1 1 1] Overlap Events
  (cast `/Game/Blueprints/BP_Player` OtherActor)
  (set `self.isInRange` true))

(event `self.ReceiveActorEndOverlap`
  (params (OtherActor :type "Actor Object Reference"))
  ;[1 1 1] Overlap Events
  (cast `/Game/Blueprints/BP_Player` OtherActor)
  (set `self.isInRange` false))

(fn `UserConstructionScript`)