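; BP_Drawbridge is a drawbridge actor that swings on its Pivot component between an open and a closed rotation.
; Each Tick picks OpenRotation or ClosedRotation from the IsOpen flag and eases the Pivot toward it with a shortest-path LerpRotator.
; The lerp uses a fixed LerpAlpha without delta time, and reads world rotation while setting relative rotation.
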(event `self.ReceiveTick`
  (params (DeltaSeconds :type "Float (single-precision)"))
  ;[1 1 1] Update
  (`|ExecutionSequence`
    (:`then_0`
      ;[1 1 1] Rotate Actor
      (if (`self.isOpen`)
        (set `self.destionationRotation` (`self.openRotation`))
        (else
          (set `self.destionationRotation` (`self.closedRotation`))))
      (`SceneComponent.K2_SetRelativeRotation` (`self.Pivot`) (`KismetMathLibrary.RLerp` (`SceneComponent.K2_GetComponentRotation` (`self.Pivot`)) (`self.destionationRotation`) (`self.lerpAlpha`) true) false false))))

(fn `UserConstructionScript`)