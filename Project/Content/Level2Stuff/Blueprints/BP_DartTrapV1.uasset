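; Dart trap prototype for Level 2, with a projectile meant to fly to a triggered position and a custom event that damages BP_Player.
; While IsTriggered is set, Tick lerps the projectile from its current location toward TriggeredPosition without sweep, giving a frame-rate-dependent ease.
; The trigger is unfinished: BeginPlay clears IsTriggered, and the overlap logic that would set it is disconnected.
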(event `CustomEvent`
  (params (OtherActor :type "Actor Object Reference"))
  (bind _asbp_player (cast `/Game/Blueprints/BP_Player` OtherActor))
  (if true
    (`GameplayStatics.ApplyDamage` _asbp_player 10.0)))

(event `self.ReceiveBeginPlay`
  (set `self.isTriggered` false))

(event `self.ReceiveTick`
  (params (DeltaSeconds :type "Float (single-precision)"))
  (if (`self.isTriggered`)
    (`SceneComponent.K2_SetWorldLocation` (`self.Projectile`) (`KismetMathLibrary.VLerp` (`SceneComponent.K2_GetComponentLocation` (`self.Projectile`)) (`self.triggeredPosition`) (`self.lerpAlpha`)) false false)))

(fn `UserConstructionScript`)