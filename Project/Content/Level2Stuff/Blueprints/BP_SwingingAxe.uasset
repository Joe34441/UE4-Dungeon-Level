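; BP_SwingingAxe is a Level 2 trap actor that swings an axe back and forth and damages the player on overlap.
; Each tick it lerps the Pivot's world rotation toward a destination, flipping between the max and min rotations once within a tolerance, so each swing eases out as it nears its end.
; The DoStuff flag gates both the swing and the damage, which applies only to BP_Player.
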(event `self.ReceiveBeginPlay`
  (set `self.destinationRotation` (`self.maxRotation`)))

(event `self.ReceiveTick`
  (params (DeltaSeconds :type "Float (single-precision)"))
  (`|ExecutionSequence`
    (:`then_0`
      (if (`self.doStuff`)
        ;[1 1 1] Rotate Axe
        (`SceneComponent.K2_SetWorldRotation` (`self.Pivot`) (`KismetMathLibrary.RLerp` (`SceneComponent.K2_GetComponentRotation` (`self.Pivot`)) (`self.destinationRotation`) (`self.lerpAlpha`) true) false false)
        (if (== (`self.destinationRotation`) (`self.maxRotation`))
          (if (== (`SceneComponent.K2_GetComponentRotation` (`self.Pivot`)) (`self.maxRotation`) :`ErrorTolerance` (`self.toleranceRotation`))
            (set `self.destinationRotation` (`self.minRotation`)))
          (elif (== (`SceneComponent.K2_GetComponentRotation` (`self.Pivot`)) (`self.minRotation`) :`ErrorTolerance` (`self.toleranceRotation`))
            (set `self.destinationRotation` (`self.maxRotation`))))))))

(event `self.ReceiveActorBeginOverlap`
  (params (OtherActor :type "Actor Object Reference"))
  (bind _asbp_player (cast `/Game/Blueprints/BP_Player` OtherActor))
  (if (`self.doStuff`)
    (`GameplayStatics.ApplyDamage` _asbp_player (`self.damage`))))

(event `self.ReceiveActorEndOverlap`
  (params (OtherActor :type "Actor Object Reference"))
  (cast `/Game/Blueprints/BP_Player` OtherActor))

(fn `UserConstructionScript`)