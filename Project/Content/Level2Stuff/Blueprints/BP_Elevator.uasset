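; Lever-operated elevator that the player toggles with the E key while overlapping the actor.
; Tick polls the key, flips the lever state and starts a cooldown timer that blocks further toggles until it expires.
; The lever state selects the Pivot rotation and Sphere location targets.
; Both ease toward them through per-frame lerps from their current transform with fixed alphas, so speed depends on frame rate.
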(event `self.ReceiveBeginPlay`
  ;[1 1 1] Start
  (if (`self.isLeverOn`)
    (set `self.destinationRotation` (`self.leverOnRotation`))
    (else
      (set `self.destinationRotation` (`self.leverOffRotation`)))))

(event `self.ReceiveTick`
  (params (DeltaSeconds :type "Float (single-precision)"))
  ;[1 1 1] Update
  (`|ExecutionSequence`
    (:`then_0`
      ;[1 1 1] Rotate Lever
      (`SceneComponent.K2_SetWorldRotation` (`self.Pivot`) (`KismetMathLibrary.RLerp` (`SceneComponent.K2_GetComponentRotation` (`self.Pivot`)) (`self.destinationRotation`) (`self.leverLerpAlpha`) true) false false)
      (if (and (`PlayerController.IsInputKeyDown` (`GameplayStatics.GetPlayerController` 0) "E") (`self.isInRange`) (`self.isWaitTimeOver`))
        (if (`self.isLeverOn`)
          (set `self.destinationRotation` (`self.leverOffRotation`))
          (set `self.isLeverOn` false)
          (else
            (set `self.destinationRotation` (`self.leverOnRotation`))
            (set `self.isLeverOn` true)))
        (set `self.isWaitTimeOver` false)))
    (:`then_1`
      ;[1 1 1] Wait Timer
      (if (`self.isWaitTimeOver`)
        _
        (elif (>= (`self.waitTimer`) (`self.totalWaitTime`))
          (set `self.waitTimer` 0.0)
          (set `self.isWaitTimeOver` true)
          (else
            (set `self.waitTimer` (+ (`GameplayStatics.GetWorldDeltaSeconds`) (`self.waitTimer`)))))))
    (:`then_2`
      ;[1 1 1] Move Elevator
      (if (`self.isLeverOn`)
        (set `self.elevatorDestinationPosition` (`self.elevatorOnPosition`))
        (else
          (set `self.elevatorDestinationPosition` (`self.elevatorOffPosition`))))
      (`SceneComponent.K2_SetWorldLocation` (`self.Sphere`) (`KismetMathLibrary.VLerp` (`SceneComponent.K2_GetComponentLocation` (`self.Sphere`)) (`self.elevatorDestinationPosition`) (`self.elevatorLerpAlpha`)) false false))))

(event `self.ReceiveActorBeginOverlap`
  (params (OtherActor :type "Actor Object Reference"))
  ;[1 1 1] Overlap Events
  (cast `/Game/Blueprints/BP_Player` OtherActor)
  (set `self.isInRange` true))

(event `self.ReceiveActorEndOverlap`
  (params (OtherActor :type "Actor Object Reference"))
  ;[1 1 1] Overlap Events
  (cast `/Game/Blueprints/BP_Player` OtherActor)
  (set `self.isInRange` false))

(fn `UserConstructionScript`)