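; BP_CorrectTileCircle is a Level 2 trigger actor that slides its Box component when BP_Player first overlaps it.
; The overlap latches IsTriggered and sets DestinationPos by adding TriggeredPosDifference to the Box location, negating that offset when MoveUp is false.
; Tick then lerps the Box from its current location toward the destination with LerpAlpha, giving a frame-rate-dependent ease-out with no reset.
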(event `self.ReceiveTick`
  (params (DeltaSeconds :type "Float (single-precision)"))
  (if (`self.isTriggered`)
    (`SceneComponent.K2_SetWorldLocation` (`self.Box`) (`KismetMathLibrary.VLerp` (`SceneComponent.K2_GetComponentLocation` (`self.Box`)) (`self.destinationPos`) (`self.lerpAlpha`)) false false)))

(event `self.ReceiveActorBeginOverlap`
  (params (OtherActor :type "Actor Object Reference"))
  (cast `/Game/Blueprints/BP_Player` OtherActor)
  (if (not (`self.isTriggered`))
    (set `self.isTriggered` true)
    (if (`self.moveUp`)
      (bind _output_get (set `self.destinationPos` (`self.triggeredPosDifference`)))
      (set `self.destinationPos` (+ _output_get (`SceneComponent.K2_GetComponentLocation` (`self.Box`))))
      (else
        (bind _output_get_2 (set `self.destinationPos` (* (`self.triggeredPosDifference`) -1.0)))
        (set `self.destinationPos` (+ _output_get_2 (`SceneComponent.K2_GetComponentLocation` (`self.Box`))))))))

(fn `UserConstructionScript`)