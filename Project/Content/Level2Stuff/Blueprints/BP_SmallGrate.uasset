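; BP_SmallGrate is a Level 2 grate that slides between an activated and an unactivated position based on its ToOpen flag.
; Each Tick picks the target position from that flag and lerps the Pivot component's world location toward it.
; Lerping from the current location by LerpAlpha gives an eased, frame-rate-dependent motion without a Timeline, sweep or teleport.
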(event `self.ReceiveTick`
  (params (DeltaSeconds :type "Float (single-precision)"))
  (`|ExecutionSequence`
    (:`then_0`
      (if (`self.toOpen`)
        (set `self.destinationPosition` (`self.activatedPosition`))
        (else
          (set `self.destinationPosition` (`self.unactivatedPosition`))))
      (`SceneComponent.K2_SetWorldLocation` (`self.Pivot`) (`KismetMathLibrary.VLerp` (`SceneComponent.K2_GetComponentLocation` (`self.Pivot`)) (`self.destinationPosition`) (`self.lerpAlpha`)) false false))))

(fn `UserConstructionScript`)