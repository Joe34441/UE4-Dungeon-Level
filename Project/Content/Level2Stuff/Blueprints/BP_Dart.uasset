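; BP_Dart is a dart trap that deals fixed damage to any BP_Player overlapping it while active.
; On Tick, an active dart lerps its Box toward Destination each frame, then deactivates and starts a cooldown on arrival.
; Once Timer reaches TotalTime, the Box snaps back to StartPosition.
; Activation and both transforms are not set in these graphs, and Timer is never reset here.
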(event `self.ReceiveActorBeginOverlap`
  (params (OtherActor :type "Actor Object Reference"))
  (if (`self.activate`)
    (bind _asbp_player (cast `/Game/Blueprints/BP_Player` OtherActor))
    (`GameplayStatics.ApplyDamage` _asbp_player 40.0)))

(event `self.ReceiveTick`
  (params (DeltaSeconds :type "Float (single-precision)"))
  (if (`self.activate`)
    (if (not (`self.cooldown`))
      (`SceneComponent.K2_SetWorldTransform` (`self.Box`) (`KismetMathLibrary.TLerp` (`SceneComponent.K2_GetComponentToWorld` (`self.Box`)) (`self.destination`) (`self.lerpAlpha`)) false false)
      (if (`KismetMathLibrary.NearlyEqual_TransformTransform` (`self.destination`) (`SceneComponent.K2_GetComponentToWorld` (`self.Box`)) 1.0 1.0 1.0)
        (set `self.activate` false)
        (set `self.cooldown` true)))
    (elif (`self.cooldown`)
      (if (>= (`self.timer`) (`self.totalTime`))
        (set `self.cooldown` false)
        (`SceneComponent.K2_SetWorldTransform` (`self.Box`) (`self.startPosition`) false false)
        (else
          (set `self.timer` (+ (`GameplayStatics.GetWorldDeltaSeconds`) (`self.timer`))))))))

(fn `UserConstructionScript`)