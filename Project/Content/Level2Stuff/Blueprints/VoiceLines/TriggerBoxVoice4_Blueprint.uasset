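; Level 2 trigger box that plays the fourth voice line, Line_4_Cue, once after the player enters it.
; Overlap with BP_Player sets a Triggered flag, and Tick then accumulates delta seconds until WaitTimer reaches TotalTime.
; A Played flag prevents repeats, and the cue plays at the world origin rather than at the trigger's location.
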(event `self.ReceiveActorBeginOverlap`
  (params (OtherActor :type "Actor Object Reference"))
  (cast `/Game/Blueprints/BP_Player` OtherActor)
  (set `self.triggered` true))

(event `self.ReceiveTick`
  (params (DeltaSeconds :type "Float (single-precision)"))
  (if (`self.triggered`)
    (if (`self.played`)
      _
      (elif (>= (`self.waitTimer`) (`self.totalTime`))
        (set `self.played` true)
        (`GameplayStatics.PlaySoundAtLocation` "/Game/Level2Stuff/VoiceLines/line_4_Cue.line_4_Cue" (0.0 0.0 0.0) (struct) 1.0 1.0 0.0 null null null)
        (else
          (set `self.waitTimer` (+ (`self.waitTimer`) (`GameplayStatics.GetWorldDeltaSeconds`))))))))

(fn `UserConstructionScript`)